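; Target actor that wanders randomly in the world X-Z plane, with no movement input along Y.
; Each Tick it adds a random offset, scaled by a fixed speed and delta time, to its current location.
; The result passes through RestrictTarget, defined outside this file, before being applied by a non-swept transform update that keeps rotation and scale.
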(event EventBeginPlay)

(event Collision|EventActorBeginOverlap
  (params (OtherActor :type Actor%20Object%20Reference)))

(event EventTick
  (params (DeltaSeconds :type Float%20%28single-precision%29))
  (bind _returnvalue (Transformation|GetActorTransform))
  (bind (_location _rotation _scale) (Math|Transform|BreakTransform _returnvalue))
  (bind _returnvalue_2 (Class|GameUtils|RestrictTarget (+ (* (Math|Vector|MakeVector (* (+ (Math|Random|RandomFloat) -0.5) 2.0) 0.0 (* (+ (Math|Random|RandomFloat) -0.5) 2.0)) (* 4e+03 DeltaSeconds)) _location)))
  (Transformation|SetActorTransform (Math|Transform|MakeTransform _returnvalue_2 _rotation _scale)))

(fn ConstructionScript)